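; Player kart pawn that maps input to throttle, steering, debug toggle and a game-pausing menu.
; Holding Left Shift swaps anti-slide, steering and damping values and enables sparks for drifting.
; R or RespawnPlayerAtNearestCP respawns the kart at the closest AI path spline point, raised along its up vector and aligned to it.
; Throttle, steering and respawn notify TutorialHud; server-call and camera snippets are left unwired.
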(event `self.ReceiveTick`
  (params (DeltaSeconds :type "Float (single-precision)"))
  (`parent.ReceiveTick` DeltaSeconds))

(event `Move forward server`
  (params (`Throttle Axis` :type "Float (double-precision)"))
  (`self.Set Throttle Input` (stale `InputAxis|Move Forward` AxisValue) :!label _label)
  (if (!= `Throttle Axis` 0.0)
    (bind _foundwidgets (`WidgetBlueprintLibrary.GetAllWidgetsOfClass` "/Game/TutorialHud.TutorialHud_C"))
    (bind _output (`|GetArrayItem` _foundwidgets))
    (`/Engine/EditorBlueprintResources/StandardMacros.IsValid` _output
      (:`Is Valid`
        (`/Game/TutorialHud.AccelComplete` _output)))))

(event `InputAxis|Move Forward`
  (params (AxisValue :type "Float (single-precision)"))
  (goto _label))

(event `move right server`
  (params (`Throttle Axis` :type "Float (double-precision)"))
  (`self.Set Steering Input` (stale `InputAxis|Move Right` AxisValue) :!label _label_2)
  (if (!= `Throttle Axis` 0.0)
    (bind _foundwidgets (`WidgetBlueprintLibrary.GetAllWidgetsOfClass` "/Game/TutorialHud.TutorialHud_C"))
    (bind _output (`|GetArrayItem` _foundwidgets))
    (`/Engine/EditorBlueprintResources/StandardMacros.IsValid` _output
      (:`Is Valid`
        (`/Game/TutorialHud.SteerComplete` _output)))))

(event `InputAxis|Move Right`
  (params (AxisValue :type "Float (single-precision)"))
  (goto _label_2))

(event `Key|E`
  (params (Key :type "Key Structure"))
  (:`Pressed`
    (`self.Toggle Debug Mode`)))

(event `InputAction|PauseButton`
  (params (Key :type "Key Structure"))
  (:`Pressed`
    (bind _returnvalue (`|CreateWidget` "/Game/pausemenu.pausemenu_C"))
    (`UserWidget.AddToViewport` _returnvalue 10)
    (`GameplayStatics.SetGamePaused` true)
    (`WidgetBlueprintLibrary.SetInputMode_UIOnlyEx` (`self.As Player Controller`) _returnvalue)
    (set `PlayerController.bShowMouseCursor` true (`self.As Player Controller`))))

(event `Key|LeftShift`
  (params (Key :type "Key Structure"))
  (:`Pressed`
    (set `self.Anti Slide` 0.0)
    (set `self.Steering Torque` 5.0)
    (set `self.Max Steer Angle` 40.0)
    (set `self.Angular Damping` 6.0)
    (`self.enableSparks`))
  (:`Released`
    (set `self.Anti Slide` 5.0)
    (set `self.Steering Torque` 6.0)
    (set `self.Max Steer Angle` 35.0)
    (set `self.Angular Damping` 3.0)
    (`self.disableSparks`)))

(event `Key|Tab`
  (params (Key :type "Key Structure")))

(event `Key|R`
  (params (Key :type "Key Structure"))
  (bind _spline (`/Game/Blueprints/BasicAI/BP_AISplinePathActor.Spline` (`self.As BP AISpline Path Actor`)))
  (bind _returnvalue (`SplineComponent.FindInputKeyClosestToWorldLocation` _spline (`self.K2_GetActorLocation`)))
  (bind _returnvalue_2 (`KismetMathLibrary.FFloor` _returnvalue))
  (bind _returnvalue_3 (`SplineComponent.GetDistanceAlongSplineAtSplinePoint` _spline _returnvalue_2))
  (bind _returnvalue_4 (+ _returnvalue_3 (* (- (`SplineComponent.GetDistanceAlongSplineAtSplinePoint` _spline (+ _returnvalue_2 1)) _returnvalue_3) (- _returnvalue (`KismetMathLibrary.Conv_IntToDouble` _returnvalue_2)))))
  (bind _returnvalue_5 (`SplineComponent.GetRotationAtDistanceAlongSpline` _spline _returnvalue_4 "World"))
  (:`Pressed`
    (`self.On Respawn` (+ (`SplineComponent.GetLocationAtDistanceAlongSpline` _spline _returnvalue_4 "World") (* (`KismetMathLibrary.GetUpVector` _returnvalue_5) (* (`.SphereRadius` (`KismetSystemLibrary.GetComponentBounds` (`self.Kart_Collision`))) 2.0))) _returnvalue_5 :!label _label_3)
    (bind _foundwidgets (`WidgetBlueprintLibrary.GetAllWidgetsOfClass` "/Game/TutorialHud.TutorialHud_C"))
    (bind _output (`|GetArrayItem` _foundwidgets))
    (`/Engine/EditorBlueprintResources/StandardMacros.IsValid` _output
      (:`Is Valid`
        (`/Game/TutorialHud.RespawnComplete` _output)))))

(event `RespawnPlayerAtNearestCP`
  (goto _label_3))

(fn `UserConstructionScript`
  (`parent.UserConstructionScript`))