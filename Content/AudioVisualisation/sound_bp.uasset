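; Audio visualisation Blueprint that scales a sphere in response to a playing sound.
; On BeginPlay it plays the sound and binds to its playback percent, which it converts to seconds using the sound's duration.
; Each update reads normalized Constant-Q data for channel 0 at that time.
; Every band value sets the same sphere's uniform scale in turn, so the last band determines the final size.
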(event `self.ReceiveBeginPlay`
  (bind _audio (`self.Audio`))
  (`AudioComponent.SetSound` _audio (`self.New Sound`))
  (set `self.Duration` (`SoundBase.Duration` (`self.New Sound`)))
  (add `AudioComponent.OnAudioPlaybackPercent` _audio (delegate `playback change`))
  (`AudioComponent.Play` (`self.Audio`) 0.0))

(event `playback change`
  (params (PlayingSoundWave :type "SoundWave Object Reference") (PlaybackPercent :type "Float (double-precision)"))
  (set `self.playback time` (* PlaybackPercent (`self.Duration`)))
  (for _array_element (`ConstantQNRT.GetNormalizedChannelConstantQAtTime` (`self.constant ref`) (`self.playback time`) 0)
    (`SceneComponent.SetWorldScale3D` (`self.Sphere`) (* (`KismetMathLibrary.Conv_DoubleToVector` _array_element) 15.0))))

(fn `UserConstructionScript`)